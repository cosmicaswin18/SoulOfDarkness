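; BP_Chest is a chest actor that shows an interaction prompt when the player is nearby.
; It creates a WB_Interact widget on BeginPlay and adds or removes it from the viewport as the player character enters or leaves the Trigger volume.
; An OpenChest event plays the chest's open animation once on its mesh; nothing in this Blueprint calls that event.
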(event `self.ReceiveBeginPlay`
  (bind _returnvalue (`|CreateWidget` "/Game/UI/WB_Interact.WB_Interact_C"))
  (set `self.Interact Widget` _returnvalue))

(event `/Game/Blueprints/Weapons/BPI_Interact.Open Chest`
  (`SkeletalMeshComponent.PlayAnimation` (`self.Chest`) "/Game/Chest/source/Chest_Anim_Armature_A_Open.Chest_Anim_Armature_A_Open" false))

(event `self.Trigger.OnComponentBeginOverlap`
  (params (OverlappedComponent :type "PrimitiveComponent Object Reference") (OtherActor :type "Actor Object Reference") (OtherComp :type "PrimitiveComponent Object Reference") (OtherBodyIndex :type Integer) (bFromSweep :type Boolean) (SweepResult :type "HitResult Structure (by ref)"))
  (if (== OtherActor (`GameplayStatics.GetPlayerCharacter` 0))
    (`UserWidget.AddToViewport` (`self.Interact Widget`) 0)))

(event `self.Trigger.OnComponentEndOverlap`
  (params (OverlappedComponent :type "PrimitiveComponent Object Reference") (OtherActor :type "Actor Object Reference") (OtherComp :type "PrimitiveComponent Object Reference") (OtherBodyIndex :type Integer))
  (if (== (`GameplayStatics.GetPlayerCharacter` 0) OtherActor)
    (`Widget.RemoveFromParent` (`self.Interact Widget`))))

(fn `UserConstructionScript`)