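; BP_Enemy_Boss is a boss enemy with its own health bar, theme music and minion summoning.
; When the player character enters BossTrigger, it adds the boss health widget, links it to BPCStats and starts the music.
; SpawnNPC checks for low health, flags the spawn in the AI blackboard and spawns several BP_Enemy at random reachable points.
; BeginPlay also captures world positions for the sword trace endpoints.
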(event `self.ReceiveBeginPlay`
  (`parent.ReceiveBeginPlay`)
  (set `self.bossStartSwordTracePos` (`SceneComponent.K2_GetComponentLocation` (`self.Boss Start Sword Trace Pos`)))
  (set `self.bossEndSwordTracePos` (`SceneComponent.K2_GetComponentLocation` (`self.Boss End Sword Trace Pos`))))

(event `self.Boss Trigger.OnComponentBeginOverlap`
  (params (OverlappedComponent :type "PrimitiveComponent Object Reference") (OtherActor :type "Actor Object Reference") (OtherComp :type "PrimitiveComponent Object Reference") (OtherBodyIndex :type Integer) (bFromSweep :type Boolean) (SweepResult :type "HitResult Structure (by ref)"))
  (cast `/Game/ThirdPerson/Blueprints/BP_ThirdPersonCharacter` OtherActor)
  (bind _returnvalue (`|CreateWidget` "/Game/UI/WB_BossHealth.WB_BossHealth_C"))
  (bind _output_get (set `self.Boss Health Widget` _returnvalue))
  (`UserWidget.AddToViewport` _output_get 0)
  (`KismetSystemLibrary.DelayUntilNextTick`)
  (`/Game/Blueprints/BPC_Stats.Set Health Progress Bar` (`self.BPC_Stats`) (`/Game/UI/WB_BossHealth.HealthBar` (`self.Boss Health Widget`)))
  (`GameplayStatics.SpawnSound2D` "/Game/FREE_Fantasy_Music_Pack/Wav/Boss_Themes/The_Weeping_King__Boss_Theme_l_Dark_l_Heavy_.The_Weeping_King__Boss_Theme_l_Dark_l_Heavy_" 1.0 1.0 0.0 null))

(event `/Game/Blueprints/AI/BPI_Enemy.Spawn NPC`
  (if (<= (`/Game/Blueprints/BPC_Stats.health` (`self.BPC_Stats`)) 150.0)
    (`BlackboardComponent.SetValueAsBool` (`AIBlueprintHelperLibrary.GetBlackboard` null) "alreadySpawned?" true)
    (for _ (range 3)
      (`|SpawnActorFromClass` "/Game/Blueprints/AI/BP_Enemy.BP_Enemy_C" (`KismetMathLibrary.MakeTransform` (`NavigationSystemV1.K2_GetRandomReachablePointInRadius` (`self.K2_GetActorLocation`) 0.0 null null)) "Undefined" "MultiplyWithRoot" null null))))

(fn `UserConstructionScript`
  (`parent.UserConstructionScript`))